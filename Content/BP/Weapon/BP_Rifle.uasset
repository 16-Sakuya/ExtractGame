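; BP_Rifle is a weapon actor that handles a single shot when OnFired is called, for an owning BP_ThirdPersonCharacter.
; It turns the owner to the camera rotation and line-traces from the camera to find the aim point.
; A BP_Bullet spawns at the muzzle facing that point, so shots converge on the screen aim.
; The owner plays a fire montage while a randomly rolled muzzle flash briefly shows.
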(event `self.OnFired`
  (bind _returnvalue (`GameplayStatics.GetPlayerCameraManager` 0))
  (bind _returnvalue_2 (`SceneComponent.K2_GetComponentLocation` (`self.muzzle`)))
  (bind _returnvalue_3 (`PlayerCameraManager.GetCameraLocation` _returnvalue))
  (bind (_relativerotation_roll _relativerotation_pitch _relativerotation_yaw) (`KismetMathLibrary.BreakRotator` (`SceneComponent.RelativeRotation` (`self.MuzzleFlash`))))
  (bind _asbp_third_person_character (cast `/Game/ThirdPerson/Blueprints/BP_ThirdPersonCharacter` (`self.GetOwner`)))
  (`self.K2_SetActorRotation` _asbp_third_person_character (`PlayerCameraManager.GetCameraRotation` (`GameplayStatics.GetPlayerCameraManager` 0)) false)
  (bind (_outhit _returnvalue_4) (`KismetSystemLibrary.LineTraceSingle` _returnvalue_3 (+ _returnvalue_3 (* (`KismetMathLibrary.GetForwardVector` (`PlayerCameraManager.GetCameraRotation` _returnvalue)) 10000.0)) "TraceTypeQuery1" false (`|MakeArray` (`self.GetOwner`))))
  (bind (_bblockinghit _binitialoverlap _time _distance _location _impactpoint _normal _impactnormal _physmat _hitactor _hitcomponent _hitbonename _bonename _hititem _elementindex _faceindex _tracestart _traceend) (`GameplayStatics.BreakHitResult` _outhit))
  (`|SpawnActorFromClass` "/Game/BP/Weapon/BP_Bullet.BP_Bullet_C" (`KismetMathLibrary.MakeTransform` _returnvalue_2 (`KismetMathLibrary.FindLookAtRotation` _returnvalue_2 (select `bool` _returnvalue_4 :`false` _traceend :`true` _location))) "AlwaysSpawn" "MultiplyWithRoot" null null)
  (bind _asbp_third_person_character_2 (cast `/Game/ThirdPerson/Blueprints/BP_ThirdPersonCharacter` (`self.GetOwner`)))
  (`Character.PlayAnimMontage` _asbp_third_person_character_2 "/Game/Characters/Mannequins/Anims/Rifle/AM_Rifle_Fire.AM_Rifle_Fire" 1.0 "None")
  (`SceneComponent.K2_SetRelativeRotation` (`self.MuzzleFlash`) (`KismetMathLibrary.MakeRotator` (`KismetMathLibrary.RandomFloatInRange` 0.0 360.0) _relativerotation_pitch _relativerotation_yaw) false false)
  (`SceneComponent.SetVisibility` (`self.MuzzleFlash`) true false)
  (`KismetSystemLibrary.Delay` 0.1)
  (`SceneComponent.SetVisibility` (`self.MuzzleFlash`) false false))

(fn `UserConstructionScript`)